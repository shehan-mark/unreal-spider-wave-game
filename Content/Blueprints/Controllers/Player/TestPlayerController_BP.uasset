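; Test player controller that announces itself on screen at BeginPlay and provides a pause toggle on the O key.
; When unpaused, pressing O creates a TESTWIDGET, adds it to the viewport as the pause menu and pauses the game.
; When paused, pressing O unpauses, removes the widget from its parent and clears the stored reference.
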(event EventBeginPlay
  (Development|PrintString "TEST GAME MODE - TEST PLAYER CONTROLLER"))

(event EventTick
  (params (DeltaSeconds :type Float%20%28single-precision%29)))

(event Input|KeyboardEvents|O
  (params (Key :type Key%20Structure :default "None"))
  (:Pressed
    (Development|PrintString "PRESSED" true true "(R=1.000000,G=0.000000,B=0.072616,A=1.000000)")
    (if (Game|IsGamePaused)
      (Game|SetGamePaused false)
      (Widget|RemovefromParent (Variables|Default|GetPauseMenu))
      (Variables|Default|SetPauseMenu 0)
      (else
        (bind _returnvalue (UserInterface|CreateWidget "/Game/Blueprints/UI/TESTWIDGET.TESTWIDGET_C" (Game|GetPlayerController 0)))
        (bind _output_get (Variables|Default|SetPauseMenu _returnvalue))
        (UserInterface|Viewport|AddtoViewport _output_get 0)
        (Game|SetGamePaused true)))))

(fn ConstructionScript)